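; A level portal that moves the player through a sequence of levels, returning to the hub at milestones.
; When the player enters its sphere, it increments the completed-level count on the GI_Main game instance.
; At the halfway point or after the final level it opens HubWhitebox with a color teleport tag.
; Otherwise it opens the next indexed level from the name array, storing that name as the tag and advancing the index.
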(event OnComponentBeginOverlap(Sphere)
  (params (OverlappedComponent :type Primitive%20Component%20Object%20Reference) (OtherActor :type Actor%20Object%20Reference) (OtherComp :type Primitive%20Component%20Object%20Reference) (OtherBodyIndex :type Integer) (bFromSweep :type Boolean) (SweepResult :type Hit%20Result%20Structure%20%28by%20ref%29))
  (if (== OtherActor (Game|Player|GetPlayerPawn 0))
    (bind _result (Math|Integer|IncrementInt (Variables|/Game/GI_Main.GI_Main_C|GetLevelsCompleted (Variables|Default|GetGI_Main%20Ref)))
      (:%20%20
        (if (== (Variables|/Game/GI_Main.GI_Main_C|GetHalfwayPoint (Variables|Default|GetGI_Main%20Ref)) _result)
          (bind _output_get (Variables|Default|SetTeleTag "Blue"))
          (Variables|/Game/GI_Main.GI_Main_C|SetTeleportTag (Variables|Default|GetGI_Main%20Ref) _output_get)
          (Game|OpenLevel(byName) "HubWhitebox")
          (Development|PrintString "Half")
          (elif (== (+ (Variables|/Game/GI_Main.GI_Main_C|GetArrayLength (Variables|Default|GetGI_Main%20Ref)) 1) (Variables|/Game/GI_Main.GI_Main_C|GetLevelsCompleted (Variables|Default|GetGI_Main%20Ref)))
            (bind _output_get_2 (Variables|Default|SetTeleTag "Green"))
            (Variables|/Game/GI_Main.GI_Main_C|SetTeleportTag (Variables|Default|GetGI_Main%20Ref) _output_get_2)
            (Game|OpenLevel(byName) "HubWhitebox")
            (else
              (bind _output_get_3 (Variables|Default|SetCurrentIndex (Variables|/Game/GI_Main.GI_Main_C|GetLevelArrayIndex (Variables|Default|GetGI_Main%20Ref))))
              (bind _arraylevelname (Utilities|ValidIndexCheck (Variables|Default|GetGI_Main%20Ref) _output_get_3))
              (Variables|Default|SetLevelName (Utilities|Array|Get(acopy) _arraylevelname (Variables|Default|GetCurrentIndex)))
              (Variables|/Game/GI_Main.GI_Main_C|SetTeleportTag (Variables|Default|GetGI_Main%20Ref) (Variables|Default|GetLevelName))
              (Math|Integer|IncrementInt (Variables|/Game/GI_Main.GI_Main_C|GetLevelArrayIndex (Variables|Default|GetGI_Main%20Ref))
                (:%20%20
                  (Game|OpenLevel(byName) (Variables|Default|GetLevelName)))))))))))

(event EventBeginPlay
  (bind _asgi_main (Utilities|Casting|CastToGI_Main (Game|GetGameInstance)))
  (bind _output_get (Variables|Default|SetGI_Main%20Ref _asgi_main))
  (Variables|Default|SetCurrentIndex (Variables|/Game/GI_Main.GI_Main_C|GetLevelArrayIndex _output_get)))

(event EventTick
  (params (DeltaSeconds :type Float%20%28single-precision%29)))

(fn ConstructionScript)