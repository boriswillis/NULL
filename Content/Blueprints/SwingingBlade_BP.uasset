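; SwingingBlade is an actor Blueprint that swings back and forth around its roll axis like a pendulum.
; Each Tick adds a frame-rate-scaled local roll from RollPerSecond, then negates that speed once the actor's roll reaches 70 degrees either way.
; The swing is constant-speed with no easing or clamping at the limits, and the current roll prints to screen every frame.
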(event EventBeginPlay)

(event Collision|EventActorBeginOverlap
  (params (OtherActor :type Actor%20Object%20Reference)))

(event EventTick
  (params (DeltaSeconds :type Float%20%28single-precision%29))
  (Transformation|AddActorLocalRotation (Math|Rotator|MakeRotator (* DeltaSeconds (Variables|Default|GetRollPerSecond)) 0.0 0.0) false false)
  (Variables|Default|SetCurrRotation (.roll (Transformation|GetActorRotation)))
  (Development|PrintString (Utilities|String|ToString(Float) (Variables|Default|GetCurrRotation)))
  (if (or (>= (Variables|Default|GetCurrRotation) 7e+01) (<= (Variables|Default|GetCurrRotation) -7e+01))
    (Variables|Default|SetCurrRotation (* (Variables|Default|GetCurrRotation) -1.0))
    (Variables|Default|SetRollPerSecond (* (Variables|Default|GetRollPerSecond) -1.0))))

(fn ConstructionScript)