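; Torch Blueprint with a Niagara fire effect that can be switched on and off.
; BeginPlay caches the fire component's relative location and sets IsTorchOn from whether that component exists.
; TorchOnandOff toggles the flame by destroying the component or adding a new Niagara component at the cached location, updating IsTorchOn to match.
; Nothing in this file calls the toggle.
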(event EventBeginPlay
  (Variables|Default|SetFireRelativeLocation (Variables|/Script/Engine.SceneComponent|GetRelativeLocation (Variables|Default|GetFireLocation)))
  (Variables|Default|GetFireLocation
    (:then
      (Variables|Default|SetIsTorchOn? true))
    (:else
      (Variables|Default|SetIsTorchOn? false))))

(event Collision|EventActorBeginOverlap
  (params (OtherActor :type Actor%20Object%20Reference)))

(event EventTick
  (params (DeltaSeconds :type Float%20%28single-precision%29)))

(fn ConstructionScript)

(fn TorchOnandOff
  (Variables|Default|GetFireLocation
    (:then
      (Components|DestroyComponent (Variables|Default|GetFireLocation))
      (Variables|Default|SetIsTorchOn? false))
    (:else
      (bind _returnvalue (AddComponent|AddNiagaraComponent false (Math|Transform|MakeTransform (Variables|Default|GetFireRelativeLocation) "0, 0, 0" "1.000000,1.000000,1.000000")))
      (Variables|Default|SetFireLocation _returnvalue)
      (Variables|Default|SetIsTorchOn? true))))