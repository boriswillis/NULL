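; Bow arrow projectile that flies on Fire, sticks into what it hits and can show a flame effect.
; Fire adds projectile movement at runtime, with strength raising speed and blending gravity between max and min, then starts the trail and collision.
; Overlapping a non-instigator removes movement, attaches the arrow, plays impact effects and pushes physics bodies with the stored launch velocity.
; The trail is removed after a short delay.
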(event OnComponentBeginOverlap(CollisionBox)
  (params (OverlappedComponent :type Primitive%20Component%20Object%20Reference) (OtherActor :type Actor%20Object%20Reference) (OtherComp :type Primitive%20Component%20Object%20Reference) (OtherBodyIndex :type Integer) (bFromSweep :type Boolean) (SweepResult :type Hit%20Result%20Structure%20%28by%20ref%29))
  (bind (_bblockinghit _binitialoverlap _time _distance _location _impactpoint _normal _impactnormal _physmat _hitactor _hitcomponent) (Collision|BreakHitResult SweepResult))
  (if (!= OtherActor (Game|GetInstigator))
    (bind _projectilemovementcomponent (Variables|Default|GetProjectileMovementComponent)
      (:then
        (Components|DestroyComponent _projectilemovementcomponent))
      (:else
        _))
    (Collision|SetCollisionEnabled (Variables|Default|GetCollisionBox) "NoCollision")
    (Transformation|AttachComponentToComponent _hitcomponent "None" "KeepWorld" "KeepWorld" "KeepWorld" true)
    (Audio|PlaySoundatLocation "/Game/Sounds/MSS_ArrowImpact.MSS_ArrowImpact" (Transformation|GetActorLocation) "0, 0, 0" 1.0 1.0 0.0 0 0 0 0)
    (Effects|SpawnEmitteratLocation (Variables|Default|GetImpactEffect) _location)
    (if (Physics|IsSimulatingPhysics _hitcomponent "None")
      (Physics|AddImpulse _hitcomponent (Variables|Default|GetVelocity) "None" true))
    (Utilities|FlowControl|Delay 1.0)
    (bind _traileffectref (Variables|Default|GetTrailEffectRef)
      (:then
        (Components|DestroyComponent _traileffectref))
      (:else))))

(event Custom|Fire
  (params (Direction :type Vector) (Strength :type Float%20%28double-precision%29))
  (Audio|PlaySoundatLocation "/Game/Sounds/MSS_ArrowWhoosh.MSS_ArrowWhoosh" (Transformation|GetActorLocation) "0, 0, 0" 1.0 1.0 0.0 0 0 0 0)
  (bind _returnvalue (AddComponent|AddProjectileMovementComponent))
  (Variables|Default|SetProjectileMovementComponent _returnvalue)
  (bind _output_get (Variables|/Script/Engine.MovementComponent|SetVelocity _returnvalue (* Direction (Math|Float|Lerp (Variables|Default|GetMinSpeed) (Variables|Default|GetMaxSpeed) Strength))))
  (Variables|Default|SetVelocity _output_get)
  (Variables|/Script/Engine.ProjectileMovementComponent|SetProjectileGravityScale _returnvalue (Math|Float|Lerp (Variables|Default|GetMaxGravity) (Variables|Default|GetMinGravity) Strength))
  (bind _returnvalue_2 (Niagara|SpawnSystemAttached (Variables|Default|GetTrailEffect) (Variables|Default|GetTrailEffectLocation) "None" "0, 0, 0" "0, 0, 0" "KeepRelativeOffset" false))
  (Variables|Default|SetTrailEffectRef _returnvalue_2)
  (Collision|SetCollisionEnabled (Variables|Default|GetCollisionBox) "QueryAndPhysics")
  (Actor|SetLifeSpan 1e+01))

(event Custom|AddFlame
  (Components|Activation|Activate (Variables|Default|GetFlameEffectLocation) false))

(event EventBeginPlay
  (Collision|SetCollisionEnabled (Variables|Default|GetCollisionBox) "NoCollision"))

(fn ConstructionScript)